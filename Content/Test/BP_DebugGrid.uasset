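; Debug actor that draws a fixed-size grid in the world when play begins, using debug lines.
; A Sequence on BeginPlay first draws a thick red rectangle outlining the 1500 by 1700 area.
; Two loops then draw thinner blue lines every 100 units along each axis, slightly below the border.
; All lines use world-space coordinates independent of the actor's transform and share one Duration variable.
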(event `self.ReceiveBeginPlay`
  (bind _duration (`self.Duration`))
  (bind _duration_2 (`self.Duration`))
  (`|ExecutionSequence`
    (:`then_0`
      (`KismetSystemLibrary.DrawDebugLine` (0.0 0.0 80.0) (1500.0 0.0 80.0) (struct :`R` 1.0 :`B` 0.169628 :`A` 1.0) _duration 30.0)
      (`KismetSystemLibrary.DrawDebugLine` (0.0 0.0 80.0) (0.0 1700.0 80.0) (struct :`R` 1.0 :`B` 0.169628 :`A` 1.0) _duration 30.0)
      (`KismetSystemLibrary.DrawDebugLine` (1500.0 0.0 80.0) (1500.0 1700.0 80.0) (struct :`R` 1.0 :`B` 0.169628 :`A` 1.0) _duration 30.0)
      (`KismetSystemLibrary.DrawDebugLine` (1500.0 1700.0 80.0) (0.0 1700.0 80.0) (struct :`R` 1.0 :`B` 0.169628 :`A` 1.0) _duration 30.0))
    (:`then_1`
      (for _index (range 18)
        (bind _returnvalue (`KismetMathLibrary.Conv_IntToDouble` (* _index 100)))
        (`KismetSystemLibrary.DrawDebugLine` (`KismetMathLibrary.MakeVector` 0.0 _returnvalue 70.0) (`KismetMathLibrary.MakeVector` 1500.0 _returnvalue 70.0) (struct :`G` 0.179102 :`B` 1.0 :`A` 1.0) _duration_2 15.0)))
    (:`then_2`
      (for _index_2 (range 16)
        (bind _returnvalue_2 (`KismetMathLibrary.Conv_IntToDouble` (* _index_2 100)))
        (`KismetSystemLibrary.DrawDebugLine` (`KismetMathLibrary.MakeVector` _returnvalue_2 0.0 70.0) (`KismetMathLibrary.MakeVector` _returnvalue_2 1700.0 70.0) (struct :`G` 0.179102 :`B` 1.0 :`A` 1.0) _duration_2 15.0)))))

(fn `UserConstructionScript`)